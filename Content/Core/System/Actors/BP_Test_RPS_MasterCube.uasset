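; Test Blueprint for a rock-paper-scissors master cube that tracks active elements in a state-to-bool map and eliminates losers.
; UpdateElements checks each non-Neutral key against the others and calls beat events, which deactivate the loser through RemoveElement and print it.
; Each removal increments MatchCount, clearing map and count at MaxMatches.
; The graph that adds CurState and triggers UpdateElements is unconnected, and BeginPlay is empty.
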(event Custom|ScissorBeatPaper
  (params (Remove :type ERPS_States%20Enum%20%28by%20ref%29 :default "Neutral"))
  (CallFunction|RemoveElement Remove))

(event Custom|PaperBeatRock
  (params (Remove :type ERPS_States%20Enum%20%28by%20ref%29 :default "Neutral"))
  (CallFunction|RemoveElement Remove))

(event Custom|RockBeatScissor
  (params (Remove :type ERPS_States%20Enum%20%28by%20ref%29 :default "Neutral"))
  (CallFunction|RemoveElement Remove))

(event EventBeginPlay)

(event EventCheckElements)

(fn ConstructionScript)

(fn UpdateElements
  (LocalVariables|SetL_Map (Variables|Default|GetmapOfStates))
  (bind _keys (Utilities|Map|Keys (LocalVariables|GetL_Map)))
  (for (_array_element _array_index) _keys
    (LocalVariables|SetL_CurState _array_element)
    (LocalVariables|SetL_curIndex _array_index)
    (if (Utilities|Enum|NotEqual(Enum) _array_element "Neutral")
      (switch Utilities|FlowControl|Switch|SwitchonERPS_States (LocalVariables|GetL_CurState)
        (:Rock
          (if (.ReturnValue (Utilities|Map|Find (LocalVariables|GetL_Map) (LocalVariables|GetL_Paper)))
            (CallFunction|PaperBeatRock (LocalVariables|GetL_Rock))
            (elif (.ReturnValue (Utilities|Map|Find (LocalVariables|GetL_Map) (LocalVariables|GetL_Scissor)))
              (CallFunction|RockBeatScissor (LocalVariables|GetL_Scissor)))))
        (:Paper
          (if (.ReturnValue (Utilities|Map|Find (LocalVariables|GetL_Map) (LocalVariables|GetL_Rock)))
            (CallFunction|PaperBeatRock (LocalVariables|GetL_Rock))
            (elif (.ReturnValue (Utilities|Map|Find (LocalVariables|GetL_Map) (LocalVariables|GetL_Scissor)))
              (CallFunction|ScissorBeatPaper (LocalVariables|GetL_Paper)))))
        (:Scissors
          (if (.ReturnValue (Utilities|Map|Find (LocalVariables|GetL_Map) (LocalVariables|GetL_Paper)))
            (CallFunction|ScissorBeatPaper (LocalVariables|GetL_Paper))
            (elif (.ReturnValue (Utilities|Map|Find (LocalVariables|GetL_Map) (LocalVariables|GetL_Rock)))
              (CallFunction|RockBeatScissor (LocalVariables|GetL_Scissor)))))))))

(fn RemoveElement
  (params (Remove :type ERPS_States%20Enum%20%28by%20ref%29 :default "Neutral"))
  (bind _mapofstates (Variables|Default|GetmapOfStates))
  (bind _keys (Utilities|Map|Keys (Variables|Default|GetmapOfStates)))
  (bind _values (Utilities|Map|Values _mapofstates))
  (if (Utilities|Array|Get(acopy) _values (Utilities|Array|FindItem _keys Remove))
    (Utilities|Map|Add _mapofstates Remove false)
    (Development|PrintString (Utilities|String|Append "Removed:" " " (Utilities|String|EnumtoString Remove)) true true "(R=1.000000,G=0.000000,B=0.000000,A=1.000000)" 5.0)
    (CallFunction|UpdateMatchCount)))

(fn UpdateMatchCount
  (bind _output_get (Variables|Default|SetmatchCount (Math|Integer|Clamp(Integer) (+ (Variables|Default|GetmatchCount) 1) 0 (Variables|Default|GetMaxMatches))))
  (if (== _output_get (Variables|Default|GetMaxMatches))
    (CallFunction|ResetGame)))

(fn ResetGame
  (Utilities|Map|Clear (Variables|Default|GetmapOfStates))
  (Variables|Default|SetmatchCount 0))